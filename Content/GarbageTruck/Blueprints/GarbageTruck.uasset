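; GarbageTruck is a truck actor that drives forward and collects grabbable objects for points.
; Each Tick it turns its Plane toward the player and sweeps along world X with a per-frame step that grows with lifetime up to a cap, unscaled by delta time.
; Box overlaps with "Grab"-tagged actors or components add their mass to the HUD score.
; Tagged actors are destroyed; tagged components are hidden and disabled, and the player drops the held item.
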(event OnComponentBeginOverlap(Box)
  (params (OverlappedComponent :type Primitive%20Component%20Object%20Reference) (OtherActor :type Actor%20Object%20Reference) (OtherComp :type Primitive%20Component%20Object%20Reference) (OtherBodyIndex :type Integer) (bFromSweep :type Boolean) (SweepResult :type Hit%20Result%20Structure%20%28by%20ref%29))
  (bind _returnvalue (Game|GetPlayerController 0))
  (bind _returnvalue_2 (HUD|GetHUD _returnvalue))
  (Utilities|FlowControl|Sequence
    (:then_0
      (if (Actor|ActorHasTag OtherActor "Grab")
        (bind _asbp_garbage_hud (Utilities|Casting|CastToBP_GarbageHUD _returnvalue_2))
        (Default|AddScore (Variables|/Game/GarbageTruck/Game/BP_GarbageHUD.BP_GarbageHUD_C|GetGarbageUI _asbp_garbage_hud) (Physics|GetMass (Actor|GetComponentbyClass OtherActor "/Script/Engine.StaticMeshComponent")))
        (Actor|DestroyActor OtherActor)))
    (:then_1
      (Utilities|IsValid OtherComp
        (:Is%20Valid
          (if (Components|ComponentHasTag OtherComp "Grab")
            (bind _asbp_garbage_hud_2 (Utilities|Casting|CastToBP_GarbageHUD _returnvalue_2))
            (Default|AddScore (Variables|/Game/GarbageTruck/Game/BP_GarbageHUD.BP_GarbageHUD_C|GetGarbageUI _asbp_garbage_hud_2) (Physics|GetMass OtherComp))
            (Rendering|SetVisibility OtherComp false false)
            (Components|Activation|SetActive OtherComp false false)
            (Variables|/Script/Engine.PrimitiveComponent|SetbGenerateOverlapEvents OtherComp false)
            (Physics|SetSimulatePhysics OtherComp false)
            (Collision|SetCollisionEnabled OtherComp "NoCollision")
            (bind _asbp_first_person_character (Utilities|Casting|CastToBP_FirstPersonCharacter (Game|Player|GetPlayerPawn 0)))
            (Default|DropItem _asbp_first_person_character)))))))

(event EventTick
  (params (DeltaSeconds :type Float%20%28single-precision%29))
  (bind _returnvalue (Transformation|GetActorLocation))
  (bind _returnvalue_2 (Actor|GetGameTimeSinceCreation))
  (bind _plane (Variables|Default|GetPlane))
  (bind _returnvalue_3 (* 0.03 _returnvalue_2))
  (bind _returnvalue_4 (+ _returnvalue_3 0.8))
  (Utilities|FlowControl|Sequence
    (:then_0
      (Transformation|SetWorldRotation _plane (Math|Rotator|FindLookatRotation (Transformation|GetWorldLocation _plane) (Transformation|GetActorLocation (Game|Player|GetPlayerPawn 0))) false false))
    (:then_1
      (if (<= _returnvalue_4 4.0)
        (Transformation|SetActorLocation (+ _returnvalue (Math|Vector|MakeVector _returnvalue_4 0.0 0.0)) true false)
        (else
          (Transformation|SetActorLocation (+ _returnvalue (Math|Vector|MakeVector 4.0 0.0 0.0)) true false))))))

(fn ConstructionScript)